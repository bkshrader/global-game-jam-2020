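; Choppable tree that grows over time and drops a BP_Log when felled, with Wood based on its growth stage.
; Construction randomizes sapling type, stage and yaw; a looping timer advances the stage, swapping the mesh and resetting stage-scaled Health.
; Interacting plays the player cursor worker's hatchet montage, then applies damage.
; At zero Health, audio and a timeline topple it before the log spawns; hovering toggles custom depth.
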(event Custom|GrowTick
  (if (< (Variables|Default|GetGrowthStage) 2)
    (bind _result (Math|Integer|IncrementInt (Variables|Default|GetGrowthStage))
      (:%20%20
        (CallFunction|SetTreeMesh (Variables|Default|GetSapling) _result)
        (Variables|Default|SetHealth (* (+ (Variables|Default|GetGrowthStage) 1) 3.0))))))

(event EventBeginPlay
  (Utilities|Time|SetTimerbyEvent (delegate Custom|GrowTick) 3e+02 true)
  (Variables|Default|SetHealth (* (+ (Variables|Default|GetGrowthStage) 1) 3.0)))

(event EventOnBeginHover
  (Rendering|SetRenderCustomDepth (Variables|Default|GetMesh) false))

(event EventOnEndHover
  (Rendering|SetRenderCustomDepth (Variables|Default|GetMesh) true))

(event Game|Damage|EventAnyDamage
  (params (Damage :type Float%20%28single-precision%29) (DamageType :type Damage%20Type%20Object%20Reference) (InstigatedBy :type Controller%20Object%20Reference) (DamageCauser :type Actor%20Object%20Reference))
  (bind _output_get (Variables|Default|SetHealth (- (Variables|Default|GetHealth) Damage)))
  (if (<= _output_get 0.0)
    (Components|Activation|Activate (Variables|Default|GetAudio) true)
    (bind _pitchover (Timeline|Felled Play)
      (:Update
        (Transformation|SetActorRotation (Math|Rotator|MakeRotator 0.0 _pitchover 0.0)))
      (:Finished
        (bind _returnvalue (Game|SpawnActorfromClass "/Game/GGJ2020/BP_Log.BP_Log_C" (Math|Conversions|ToTransform(Vector) (+ (Transformation|GetActorLocation) "0, 0,50.000000")) "AdjustIfPossibleButAlwaysSpawn" 0 0))
        (Variables|/Game/GGJ2020/BP_Log.BP_Log_C|SetWood _returnvalue (+ (Variables|Default|GetGrowthStage) 1))
        (Actor|DestroyActor)))))

(event EventOnBeginInteract
  (bind _asbp_player_cursor (Utilities|Casting|CastToBP_PlayerCursor (Game|Player|GetPlayerPawn 0))
    (:then
      (Animation|Montage|PlayMontage (Variables|/Script/Engine.Character|GetMesh (Variables|/Game/GGJ2020/BP_PlayerCursor.BP_PlayerCursor_C|GetWorker _asbp_player_cursor)) "/Game/GGJ2020/AM_HatchetSwing.AM_HatchetSwing"
        (:OnCompleted
          _)))
    (:CastFailed
      _))
  (Game|Damage|ApplyDamage self 1.0 0 0))

(fn ConstructionScript
  (bind _returnvalue (Math|Random|RandomInteger 2))
  (bind _returnvalue_2 (* _returnvalue 3.0))
  (bind _returnvalue_3 (Math|Float|Truncate _returnvalue_2))
  (Variables|Default|SetSapling _returnvalue_3)
  (bind _output_get (Variables|Default|SetGrowthStage (Math|Random|RandomInteger 3)))
  (CallFunction|SetTreeMesh _output_get _returnvalue_3)
  (Transformation|SetActorRotation (Math|Rotator|MakeRotator 0.0 0.0 (Math|Random|RandomFloatinRange 0.0 6.28))))

(fn SetTreeMesh
  (params (SaplingIndex :type Integer) (GrowthStage :type Integer))
  (Components|StaticMesh|SetStaticMesh (Variables|Default|GetMesh) (Utilities|Array|Get(acopy) (Variables|Default|GetTrees) (+ SaplingIndex GrowthStage)))
  (return))