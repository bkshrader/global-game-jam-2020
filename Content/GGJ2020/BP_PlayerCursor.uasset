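; Player cursor actor for a GGJ2020 game that spawns and commands an AI worker.
; Each tick a vertical line trace snaps a cursor component to the surface below, aligned to its normal.
; Overlaps track the hovered BPI_Interactable and send it hover begin and end messages.
; The Action input writes either the hovered actor or the cursor location into the worker's blackboard as its target, clearing the other key.
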(event Collision|EventActorBeginOverlap
  (params (OtherActor :type Actor%20Object%20Reference))
  (if (Utilities|DoesObjectImplementInterface OtherActor "/Game/GGJ2020/BPI_Interactable.BPI_Interactable_C")
    (bind _output_get (Variables|Default|SetHoveredInteractable OtherActor))
    (Class|BPIInteractable|OnBeginHover(Message) _output_get)))

(event Collision|EventActorEndOverlap
  (params (OtherActor :type Actor%20Object%20Reference))
  (if (Utilities|DoesObjectImplementInterface OtherActor "/Game/GGJ2020/BPI_Interactable.BPI_Interactable_C")
    (Utilities|IsValid (Variables|Default|GetHoveredInteractable)
      (:Is%20Valid
        (Class|BPIInteractable|OnEndHover(Message) (Variables|Default|GetHoveredInteractable))
        (Variables|Default|SetHoveredInteractable 0)))))

(event EventTick
  (params (DeltaSeconds :type Float%20%28single-precision%29))
  (bind _returnvalue (Transformation|GetActorLocation))
  (bind _outhit (Collision|LineTraceByChannel (+ _returnvalue "0, 0,1000.000000") (- _returnvalue "0, 0,1000.000000") "TraceTypeQuery1" false 0 "None"))
  (Transformation|SetWorldLocationAndRotation (Variables|Default|GetCursorToWorld) (.Location (Collision|BreakHitResult _outhit)) (Math|Rotator|MakeRotationfromAxes (.ImpactNormal (Collision|BreakHitResult _outhit)) "0, 0, 0" "0, 0, 0") false false))

(event EventBeginPlay
  (bind _returnvalue (Game|SpawnActorfromClass "/Game/GGJ2020/BP_PlayerWorker.BP_PlayerWorker_C" (Transformation|GetActorTransform) "Undefined" 0 0))
  (Variables|Default|SetWorker _returnvalue))

(event Input|ActionEvents|InputActionAction
  (params (Key :type Key%20Structure :default "None"))
  (bind _hoveredinteractable (Variables|Default|GetHoveredInteractable))
  (:Pressed
    (Utilities|IsValid _hoveredinteractable
      (:Is%20Valid
        (AI|Components|Blackboard|SetValueasObject (AI|GetBlackboard (Variables|Default|GetWorker)) (Utilities|Name|MakeLiteralName "TargetActor") _hoveredinteractable)
        (AI|Components|Blackboard|SetValueasVector (AI|GetBlackboard (Variables|Default|GetWorker)) (Utilities|Name|MakeLiteralName "TargetLocation") "0, 0, 0"))
      (:Is%20Not%20Valid
        (AI|Components|Blackboard|SetValueasVector (AI|GetBlackboard (Variables|Default|GetWorker)) (Utilities|Name|MakeLiteralName "TargetLocation") (Transformation|GetWorldLocation (Variables|Default|GetCursorToWorld)))
        (AI|Components|Blackboard|SetValueasObject (AI|GetBlackboard (Variables|Default|GetWorker)) (Utilities|Name|MakeLiteralName "TargetActor") 0)))))

(fn ConstructionScript)