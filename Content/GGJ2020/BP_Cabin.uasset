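; BP_Cabin is an interactable cabin build site that the player completes by delivering wood to win the game.
; Interacting takes wood from BP_PlayerCursor, lowers WoodNeeded and updates the count text, which the construction script initialises.
; At zero, it relabels itself "Cabin", removes the wood labels and shows WBP_WinScreen with UI-only input.
; Hover toggles the mesh's custom depth, turning it off while hovered and on afterwards.
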(event EventOnBeginHover
  (Rendering|SetRenderCustomDepth (Variables|Default|GetMesh) false))

(event EventOnEndHover
  (Rendering|SetRenderCustomDepth (Variables|Default|GetMesh) true))

(event EventOnBeginInteract
  (bind _returnvalue (Game|GetPlayerController 0))
  (bind _asbp_player_cursor (Utilities|Casting|CastToBP_PlayerCursor (Game|Player|GetPlayerPawn 0)))
  (bind _woodtaken (Default|TakeWood _asbp_player_cursor (Variables|Default|GetWoodNeeded)))
  (bind _output_get (Variables|Default|SetWoodNeeded (- (Variables|Default|GetWoodNeeded) _woodtaken)))
  (Rendering|Components|TextRender|SetText (Variables|Default|GetWoodAmount) (Utilities|Text|ToText(Integer) _output_get))
  (if (<= _output_get 0)
    (Rendering|Components|TextRender|SetText (Variables|Default|GetNameLabel) (Utilities|Text|MakeLiteralText "Cabin"))
    (Components|DestroyComponent (Variables|Default|GetWoodLabel))
    (Components|DestroyComponent (Variables|Default|GetWoodAmount))
    (bind _returnvalue_2 (UserInterface|CreateWidget "/Game/GGJ2020/WBP_WinScreen.WBP_WinScreen_C" (Game|GetPlayerController 0)))
    (UserInterface|Viewport|AddtoViewport _returnvalue_2 0)
    (Variables|/Script/Engine.PlayerController|SetbShowMouseCursor _returnvalue true)
    (Input|SetInputModeUIOnly _returnvalue _returnvalue_2 "DoNotLock")))

(fn ConstructionScript
  (Rendering|Components|TextRender|SetText (Variables|Default|GetWoodAmount) (Utilities|Text|ToText(Integer) (Variables|Default|GetWoodNeeded))))