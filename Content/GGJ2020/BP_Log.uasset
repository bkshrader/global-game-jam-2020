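; Harvestable log that gives the player wood when interacted with through BP_PlayerCursor.
; Interaction plays a hatchet swing montage on the cursor's Worker mesh.
; On montage completion it gives the cursor one wood, decrements its own Wood count and destroys itself when depleted.
; Hover events toggle the mesh's custom depth, switching it off on hover begin and on at hover end.
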(event EventOnBeginInteract
  (bind _asbp_player_cursor (Utilities|Casting|CastToBP_PlayerCursor (Game|Player|GetPlayerPawn 0)))
  (Animation|Montage|PlayMontage (Variables|/Script/Engine.Character|GetMesh (Variables|/Game/GGJ2020/BP_PlayerCursor.BP_PlayerCursor_C|GetWorker _asbp_player_cursor)) "/Game/GGJ2020/AM_HatchetSwing.AM_HatchetSwing"
    (:OnCompleted
      (Default|GiveWood _asbp_player_cursor 1)
      (bind _result (Math|Integer|DecrementInt (Variables|Default|GetWood))
        (:%20%20
          (if (<= _result 0)
            (Actor|DestroyActor)))))))

(event EventOnBeginHover
  (Rendering|SetRenderCustomDepth (Variables|Default|GetMesh) false))

(event EventOnEndHover
  (Rendering|SetRenderCustomDepth (Variables|Default|GetMesh) true))

(event EventBeginPlay)

(fn ConstructionScript)